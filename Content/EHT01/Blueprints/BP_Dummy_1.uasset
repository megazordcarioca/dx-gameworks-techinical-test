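; Enemy dummy character that chases and shoots the player, with health and a floating health widget.
; It stays still until PawnSensing spots a pawn, then moves toward the player via AIMoveTo, firing BP_Projectile after a delay with a montage.
; TakeDamage adds player score, lowers clamped health, triggers TakeStun and destroys the dummy at zero.
; BeginPlay also calls TakeDamage before refreshing the widget, which AnyDamage updates after its parent handler.
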(event OnSeePawn(PawnSensing)
  (params (Pawn :type Pawn%20Object%20Reference))
  ;[1 1 1] AI Detect System
  (bind _output_get (Variables|Default|SetPlayerIsNearby true))
  (if _output_get
    (CallFunction|FollowPlayer)))

(event Custom|Follow%20Player
  ;[1 1 1] Movement AI System
  (Variables|Default|SetcanAttack true)
  (if (Variables|Default|GetPlayerIsNearby)
    (AI|AIMoveTo self "0, 0, 0" (Game|GetPlayerCharacter 0) 5.0 false
      (:then
        _)
      (:OnSuccess
        _))
    (if (Variables|Default|GetcanAttack)
      (CallFunction|ShotonPlayer 1.0))))

(event Custom|Shot%20on%20Player
  (params (shotFrequency :type Float%20%28double-precision%29))
  ;[1 1 1] Shot on Player System
  (if (Variables|Default|GetPlayerIsNearby)
    (Utilities|FlowControl|Delay shotFrequency)
    (Animation|PlayAnimMontage "/Game/FirstPersonArms/Animations/FirstPersonFire_Montage.FirstPersonFire_Montage" 1.0 "None")
    (Game|SpawnActorfromClass "/Game/EHT01/Blueprints/BP_Projectile.BP_Projectile_C" (Transformation|GetWorldTransform (Variables|Default|GetArrowProjectile)) "Undefined" 0 0.0 0)
    (else
      (Variables|Default|SetcanAttack false))))

(event EventBeginPlay
  (bind _asdummy_uisystem (Utilities|Casting|CastToDummyUISystem (UserInterface|GetWidget (Variables|Default|GetWidgetEnemyComponent))))
  (bind _output_get (Variables|Default|SetDummyUISystem _asdummy_uisystem))
  (CallFunction|TakeDamage 1e+01)
  (Default|UpdateEnemyHealth _output_get (Variables|Default|GetcurrentEnemyHealth)))

(event Collision|EventActorBeginOverlap
  (params (OtherActor :type Actor%20Object%20Reference)))

(event EventTick
  (params (DeltaSeconds :type Float%20%28single-precision%29))
  (if (not (Variables|Default|GetPlayerIsNearby))
    (Components|Movement|StopMovementImmediately (Variables|Character|GetCharacterMovement))))

(event EventTakeDamage
  (params (DamageValue :type Float%20%28double-precision%29))
  ;[1 1 1] Health System
  (bind _asbp_first_person_character (Utilities|Casting|CastToBP_FirstPersonCharacter (Game|GetPlayerCharacter 0)))
  (Variables|/Game/EHT01/Blueprints/BP_FirstPersonCharacter.BP_FirstPersonCharacter_C|SetscoreValue _asbp_first_person_character (+ (Variables|/Game/EHT01/Blueprints/BP_FirstPersonCharacter.BP_FirstPersonCharacter_C|GetscoreValue _asbp_first_person_character) 1e+01))
  (bind _output_get (Variables|Default|SetcurrentEnemyHealth (Math|Float|Clamp(Float) (- (Variables|Default|GetcurrentEnemyHealth) DamageValue) 0.0 (Variables|Default|GetmaxEnemyHealth))))
  (bind _output_get_2 (Variables|Default|SetisEnemyDamaged true))
  (if _output_get_2
    (CallFunction|TakeStun 2e+01)
    (bind _output_get_3 (Variables|Default|SetcurrentEnemyHealth _output_get))
    (bind _output_get_4 (Variables|Default|SetisDummyDead (== _output_get_3 0.0)))
    (if _output_get_4
      (bind _returnvalue (Actor|GetActorOfClass "BP_Dummy_1_C"))
      (Utilities|IsValid _returnvalue
        (:Is%20Valid
          (Actor|DestroyActor self))))))

(event Game|Damage|EventAnyDamage
  (params (Damage :type Float%20%28single-precision%29) (DamageType :type Damage%20Type%20Object%20Reference) (InstigatedBy :type Controller%20Object%20Reference) (DamageCauser :type Actor%20Object%20Reference))
  (|CallParentFunction Damage DamageType InstigatedBy DamageCauser)
  (Default|UpdateEnemyHealth (Variables|Default|GetDummyUISystem) (Variables|Default|GetcurrentEnemyHealth)))

(fn ConstructionScript)